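; Vertical moving platform Blueprint that travels between its placed location and a point Height units above it.
; BeginPlay stores the start location, computes the raised target, sets the Moveup timeline's play rate from Speed and starts it.
; Each timeline update lerps the actor's location between the two points using the MoveUp track, without sweeping for collisions.
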(event `self.ReceiveBeginPlay`
  ;[1 1 1] up / down platform
  (bind _output_get (set `self.originalLocation` (`self.K2_GetActorLocation`)))
  (set `self.newLocation` (+ _output_get (`KismetMathLibrary.MakeVector` 0.0 0.0 (`self.height`))))
  (`TimelineComponent.SetPlayRate` (`self.Moveup`) (`self.speed`))
  (bind (_direction _moveup) (`Timeline|Moveup` :!via `PlayFromStart`)
    (:`Update`
      (`self.K2_SetActorLocation` (`KismetMathLibrary.VLerp` (`self.originalLocation`) (`self.newLocation`) _moveup)))))

(fn `UserConstructionScript`)