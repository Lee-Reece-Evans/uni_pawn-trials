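; BP_Gate is a gate actor that removes itself when the player reaches it while it is unlocked.
; An overlap on its sphere checks for the player character and the Locked flag.
; On success it assigns the ParticleEffect template to its particle component, waits briefly, then destroys the actor.
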(event `self.Sphere.OnComponentBeginOverlap`
  (params (OverlappedComponent :type "PrimitiveComponent Object Reference") (OtherActor :type "Actor Object Reference") (OtherComp :type "PrimitiveComponent Object Reference") (OtherBodyIndex :type Integer) (bFromSweep :type Boolean) (SweepResult :type "HitResult Structure (by ref)"))
  ;[1 1 1] when gate unlocked play partcle and delete actor
  (if (and (== OtherActor (`GameplayStatics.GetPlayerCharacter` 0)) (not (`self.locked`)))
    (`ParticleSystemComponent.SetTemplate` (`self.ParticleSystem`) (`self.Particle_Effect`))
    (`KismetSystemLibrary.Delay` 3.0)
    (`self.K2_DestroyActor`)))

(fn `UserConstructionScript`)