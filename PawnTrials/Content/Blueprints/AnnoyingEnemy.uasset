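; AnnoyingEnemy is a side-scroller enemy or hazard that deals continuous damage to the player while overlapping its Box component.
; Begin overlap confirms the controlled pawn, casts it to SideScrollerCharacterTwo and applies damage immediately.
; ContinueDamage repeats through a looping timer at DamageRate, re-set on every hit.
; End overlap clears that timer without checking which actor left.
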(event `Continue Damage`
  ;[1 1 1] continious damage
  (`/Game/Blueprints/SideScrollerCharacterTwo.DamagePlayer` (stale `self.Box.OnComponentBeginOverlap` _asside_scroller_character_two) (`self.Damage`) :!label _label)
  (bind _returnvalue (`KismetSystemLibrary.K2_SetTimerDelegate` (delegate `Continue Damage`) (`self.Damage Rate`) true))
  (set `self.Timer Handler` _returnvalue))

(event `self.Box.OnComponentBeginOverlap`
  (params (OverlappedComponent :type "PrimitiveComponent Object Reference") (OtherActor :type "Actor Object Reference") (OtherComp :type "PrimitiveComponent Object Reference") (OtherBodyIndex :type Integer) (bFromSweep :type Boolean) (SweepResult :type "HitResult Structure (by ref)"))
  (bind _returnvalue (`Controller.K2_GetPawn` (`GameplayStatics.GetPlayerController` 0)))
  ;[1 1 1] continious damage
  (if (== OtherActor _returnvalue)
    (bind _asside_scroller_character_two (cast `/Game/Blueprints/SideScrollerCharacterTwo` _returnvalue))
    (goto _label)))

(event `self.Box.OnComponentEndOverlap`
  (params (OverlappedComponent :type "PrimitiveComponent Object Reference") (OtherActor :type "Actor Object Reference") (OtherComp :type "PrimitiveComponent Object Reference") (OtherBodyIndex :type Integer))
  ;[1 1 1] Stop Damage
  (`KismetSystemLibrary.K2_ClearAndInvalidateTimerHandle` (`self.Timer Handler`)))

(fn `UserConstructionScript`)