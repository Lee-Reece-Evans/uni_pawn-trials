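; Projectile bullet that damages enemy AI on hit and expires after a short lifespan.
; The construction script feeds ProjectileSpeed into the projectile movement's initial speed.
; Sphere overlaps ignore the player's pawn and components tagged "interact"; other overlaps spawn a metal impact effect and destroy the bullet.
; If the overlapped actor is a BP_enemyAI, its DamageAI receives the bullet's Damage.
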(event `self.ReceiveBeginPlay`
  ;[1 1 1] set bullet lifetime
  (`self.SetLifeSpan` 5.0))

(event `PlayImpact`
  ;[1 1 1] play impact effect
  (`GameplayStatics.SpawnEmitterAtLocation` "/Game/SciFiWeapDark/FX/Particles/P_Impact_Metal_Medium_Light.P_Impact_Metal_Medium_Light" (`SceneComponent.K2_GetComponentLocation` (`self.Sphere`)))
  (`self.K2_DestroyActor`))

(event `self.Sphere.OnComponentBeginOverlap`
  (params (OverlappedComponent :type "PrimitiveComponent Object Reference") (OtherActor :type "Actor Object Reference") (OtherComp :type "PrimitiveComponent Object Reference") (OtherBodyIndex :type Integer) (bFromSweep :type Boolean) (SweepResult :type "HitResult Structure (by ref)"))
  ;[1 1 1] Comment
  (`/Engine/EditorBlueprintResources/StandardMacros.IsValid` OtherActor
    (:`Is Valid`
      (if (and (!= OtherActor (`Controller.K2_GetPawn` (`GameplayStatics.GetPlayerController` 0))) (not (`ActorComponent.ComponentHasTag` OtherComp "interact")))
        (`self.PlayImpact`)
        (bind _asbp_enemy_ai (cast `/Game/Blueprints/BP_enemyAI` OtherActor))
        (`/Game/Blueprints/BP_enemyAI.DamageAI` _asbp_enemy_ai (`self.Damage`))))
    (:`Is Not Valid`
      (`self.PlayImpact`))))

(fn `UserConstructionScript`
  (set `ProjectileMovementComponent.InitialSpeed` (`self.Projectile Speed`) (`self.ProjectileMovement`)))