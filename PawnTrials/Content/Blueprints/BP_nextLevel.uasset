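; Level exit trigger that ends the level when the player character overlaps its box.
; It sets GameOver on the game mode, saves a new best score or best time for the level through the game instance, and carries the total score over as the next starting score.
; It then slows time, disables input and shows the next-level menu, or the end menu on the final level.
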(event `self.Box.OnComponentBeginOverlap`
  (params (OverlappedComponent :type "PrimitiveComponent Object Reference") (OtherActor :type "Actor Object Reference") (OtherComp :type "PrimitiveComponent Object Reference") (OtherBodyIndex :type Integer) (bFromSweep :type Boolean) (SweepResult :type "HitResult Structure (by ref)"))
  (bind _game_instance (`self.game instance`))
  (bind _game_instance_2 (`self.game instance`))
  (bind _level_score (`self.level score`))
  (bind _level_time (`self.level time`))
  (bind _best_score (`/Game/Blueprints/GameMode/MyGameInstance.best score` _game_instance))
  (bind _best_time (`/Game/Blueprints/GameMode/MyGameInstance.best time` _game_instance))
  (bind _level_num (`/Game/Blueprints/GameMode/MyGameInstance.level num` _game_instance))
  (bind _output (`|GetArrayItem` _best_time _level_num))
  ;[1 1 1] transition to next level. take note of total score to use as starting score for next level. check level score and time to save as stats
  (if (== OtherActor (`GameplayStatics.GetPlayerCharacter` 0))
    (`|ExecutionSequence`
      (:`then_0`
        (bind _asmy_game_instance (cast `/Game/Blueprints/GameMode/MyGameInstance` (`GameplayStatics.GetGameInstance`)))
        (set `self.game instance` _asmy_game_instance))
      (:`then_1`
        (bind _asmy_game_mode (cast `/Game/Blueprints/GameMode/MyGameMode` (`GameplayStatics.GetGameMode`)))
        (set `/Game/Blueprints/GameMode/MyGameMode.GameOver` true _asmy_game_mode)
        (set `self.level score` (`/Game/Blueprints/GameMode/MyGameMode.Score` _asmy_game_mode))
        (set `self.level time` (`KismetMathLibrary.FFloor` (`/Game/Blueprints/GameMode/MyGameMode.GameTime` _asmy_game_mode)))
        (`|ExecutionSequence`
          (:`then_0`
            (`|ExecutionSequence`
              (:`then_0`
                (`/Engine/EditorBlueprintResources/StandardMacros.CompareInt` _level_score (`|GetArrayItem` _best_score _level_num)
                  (:`>`
                    (`KismetArrayLibrary.Array_Set` _best_score _level_num _level_score true))))
              (:`then_1`
                (`/Engine/EditorBlueprintResources/StandardMacros.CompareInt` _output
                  (:`>`
                    (`/Engine/EditorBlueprintResources/StandardMacros.CompareInt` _level_time _output
                      (:`<`
                        _)))
                  (:`==`
                    _))
                (`KismetArrayLibrary.Array_Set` _best_time _level_num _level_time true)))
            (`/Game/Blueprints/GameMode/MyGameInstance.save` (`self.game instance`)))
          (:`then_1`
            (set `/Game/Blueprints/GameMode/MyGameInstance.StartingScore` (`/Game/Blueprints/GameMode/MyGameInstance.TotalScore` _game_instance_2) _game_instance_2)
            (`GameplayStatics.SetGlobalTimeDilation` 0.2)
            (`KismetSystemLibrary.Delay` 0.2)
            (`self.DisableInput` (`GameplayStatics.GetPlayerPawn` 0) (`GameplayStatics.GetPlayerController` 0))
            (if (== (`/Game/Blueprints/GameMode/MyGameInstance.level num` _game_instance_2) (`self.end level number`))
              (`self.end level`)
              (else
                (set `/Game/Blueprints/GameMode/MyGameInstance.next level ref` (`self.nextLevel`) _game_instance_2)
                (`self.next level`)))))))))

(fn `end level`
  (bind _returnvalue (`GameplayStatics.GetPlayerController` 0))
  (bind _returnvalue_2 (`|CreateWidget` "/Game/UI/Widget_endlevelmenu.Widget_endlevelmenu_C" _returnvalue))
  (`UserWidget.AddToViewport` _returnvalue_2 0)
  (`WidgetBlueprintLibrary.SetInputMode_UIOnlyEx` _returnvalue _returnvalue_2)
  (set `PlayerController.bShowMouseCursor` true _returnvalue))

(fn `next level`
  (bind _returnvalue (`GameplayStatics.GetPlayerController` 0))
  (bind _returnvalue_2 (`|CreateWidget` "/Game/UI/Widget_nextlevelmenu.Widget_nextlevelmenu_C" _returnvalue))
  (`UserWidget.AddToViewport` _returnvalue_2 0)
  (`WidgetBlueprintLibrary.SetInputMode_UIOnlyEx` _returnvalue _returnvalue_2)
  (set `PlayerController.bShowMouseCursor` true _returnvalue))

(fn `UserConstructionScript`)