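; Projectile, named for traps, that damages the side-scroller player character when its sphere overlaps them.
; The construction script feeds ProjectileSpeed into the projectile movement's initial speed.
; On overlap it calls DamagePlayer on the player or stops at other actors, passing through those tagged "dontBlockProj".
; Impacts spawn a fire particle effect and an attenuated sound at the sphere, then destroy the actor.
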(event `PlayImapact`
  (bind _returnvalue (`SceneComponent.K2_GetComponentLocation` (`self.Sphere`)))
  ;[1 1 1] impact effect
  (`GameplayStatics.SpawnEmitterAtLocation` "/Game/InfinityBladeEffects/Effects/FX_Combat_Base/Impact/P_Impact_Player_Fire_Strong.P_Impact_Player_Fire_Strong" _returnvalue)
  (`GameplayStatics.PlaySoundAtLocation` "/Game/SciFiWeapDark/Sound/SniperRifle/SniperRifle_ImpactBody_Cue.SniperRifle_ImpactBody_Cue" _returnvalue (struct) 1.0 1.0 0.0 "/Game/SciFiWeapDark/Sound/Attenuation/WeaponHandling_att.WeaponHandling_att" null null)
  (`self.K2_DestroyActor`))

(event `self.Sphere.OnComponentBeginOverlap`
  (params (OverlappedComponent :type "PrimitiveComponent Object Reference") (OtherActor :type "Actor Object Reference") (OtherComp :type "PrimitiveComponent Object Reference") (OtherBodyIndex :type Integer) (bFromSweep :type Boolean) (SweepResult :type "HitResult Structure (by ref)"))
  (bind _returnvalue (`GameplayStatics.GetPlayerCharacter` 0))
  ;[1 1 1] deal damage
  (`/Engine/EditorBlueprintResources/StandardMacros.IsValid` OtherActor
    (:`Is Valid`
      (if (== OtherActor _returnvalue)
        (bind _asside_scroller_character_two (cast `/Game/Blueprints/SideScrollerCharacterTwo` _returnvalue))
        (`/Game/Blueprints/SideScrollerCharacterTwo.DamagePlayer` _asside_scroller_character_two (`self.Damage`))
        (`self.PlayImapact`)
        (elif (not (`self.ActorHasTag` OtherActor "dontBlockProj"))
          (`self.PlayImapact`))))
    (:`Is Not Valid`
      (`self.PlayImapact`))))

(fn `UserConstructionScript`
  (set `ProjectileMovementComponent.InitialSpeed` (`self.Projectile Speed`) (`self.ProjectileMovement`)))