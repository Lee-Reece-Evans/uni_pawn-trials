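; BP_spiketrap is a spike trap hazard that moves vertically and damages the player on contact.
; On BeginPlay a timeline, with play rate set by Speed, lerps the actor between its start location and a point offset upward by Height.
; When the local player overlaps its Box, it casts to SideScrollerCharacterTwo and calls DamagePlayer with the Damage value.
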(event `self.ReceiveBeginPlay`
  ;[1 1 1] spike trap movement
  (bind _output_get (set `self.originalLocation` (`self.K2_GetActorLocation`)))
  (set `self.newLocation` (+ _output_get (`KismetMathLibrary.MakeVector` 0.0 0.0 (`self.height`))))
  (`TimelineComponent.SetPlayRate` (`self.move`) (`self.speed`))
  (bind (_direction _moveup) (`Timeline|move` :!via `PlayFromStart`)
    (:`Update`
      (`self.K2_SetActorLocation` (`KismetMathLibrary.VLerp` (`self.originalLocation`) (`self.newLocation`) _moveup)))))

(event `self.Box.OnComponentBeginOverlap`
  (params (OverlappedComponent :type "PrimitiveComponent Object Reference") (OtherActor :type "Actor Object Reference") (OtherComp :type "PrimitiveComponent Object Reference") (OtherBodyIndex :type Integer) (bFromSweep :type Boolean) (SweepResult :type "HitResult Structure (by ref)"))
  ;[1 1 1] spike trap damage
  (if (== OtherActor (`GameplayStatics.GetPlayerCharacter` 0))
    (bind _asside_scroller_character_two (cast `/Game/Blueprints/SideScrollerCharacterTwo` OtherActor))
    (`/Game/Blueprints/SideScrollerCharacterTwo.DamagePlayer` _asside_scroller_character_two (`self.Damage`))))

(fn `UserConstructionScript`)