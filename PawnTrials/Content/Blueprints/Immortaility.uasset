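; Immortality pickup that makes the player's side-scroller character immune to damage when touched.
; When the controlled pawn overlaps its Box, it clears TakeDamage on SideScrollerCharacterTwo, calls that character's DisableImmunity, then destroys itself.
; A second sequence branch spawns a BP_shield at the pickup's transform, after the destroy call.
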(event `self.Box.OnComponentBeginOverlap`
  (params (OverlappedComponent :type "PrimitiveComponent Object Reference") (OtherActor :type "Actor Object Reference") (OtherComp :type "PrimitiveComponent Object Reference") (OtherBodyIndex :type Integer) (bFromSweep :type Boolean) (SweepResult :type "HitResult Structure (by ref)"))
  (bind _returnvalue (`Controller.K2_GetPawn` (`GameplayStatics.GetPlayerController` 0)))
  (if (== OtherActor _returnvalue)
    (`|ExecutionSequence`
      (:`then_0`
        (bind _asside_scroller_character_two (cast `/Game/Blueprints/SideScrollerCharacterTwo` _returnvalue))
        (set `/Game/Blueprints/SideScrollerCharacterTwo.TakeDamage?` false _asside_scroller_character_two)
        (`/Game/Blueprints/SideScrollerCharacterTwo.DisableImmunity` _asside_scroller_character_two)
        (`self.K2_DestroyActor`))
      (:`then_1`
        (`|SpawnActorFromClass` "/Game/Blueprints/BP_shield.BP_shield_C" (`self.GetTransform`) "Undefined" "OverrideRootScale" null null)))))

(fn `UserConstructionScript`)