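; Health pickup actor that restores health to the side-scroller player character on touch.
; When its Box is overlapped by the player-controlled pawn, it casts that pawn to SideScrollerCharacterTwo and checks whether health is below maximum.
; If so, it adds the restore amount, clamped to the character's maximum, and destroys itself; at full health the pickup stays in the world.
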(event `self.Box.OnComponentBeginOverlap`
  (params (OverlappedComponent :type "PrimitiveComponent Object Reference") (OtherActor :type "Actor Object Reference") (OtherComp :type "PrimitiveComponent Object Reference") (OtherBodyIndex :type Integer) (bFromSweep :type Boolean) (SweepResult :type "HitResult Structure (by ref)"))
  (bind _returnvalue (`Controller.K2_GetPawn` (`GameplayStatics.GetPlayerController` 0)))
  ;[1 1 1] add health to player if damaged and not more than max health after added restore amount
  (if (== OtherActor _returnvalue)
    (bind _asside_scroller_character_two (cast `/Game/Blueprints/SideScrollerCharacterTwo` _returnvalue))
    (bind _playerhealth (`/Game/Blueprints/SideScrollerCharacterTwo.PlayerHealth` _asside_scroller_character_two))
    (bind _maxhealth (`/Game/Blueprints/SideScrollerCharacterTwo.MaxHealth` _asside_scroller_character_two))
    (if (< _playerhealth _maxhealth)
      (set `/Game/Blueprints/SideScrollerCharacterTwo.PlayerHealth` (`KismetMathLibrary.FClamp` (+ _playerhealth (`self.Retore Amount`)) 0.0 _maxhealth) _asside_scroller_character_two)
      (`self.K2_DestroyActor`))))

(fn `UserConstructionScript`)