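; A moving platform that slides side to side along the world X axis, starting when play begins.
; On BeginPlay it stores its starting location and derives a target offset by XMovement.
; The Moveside timeline, with play rate set by Speed, drives a vector lerp between the two points through its MoveUp track and sets the actor location without sweeping.
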(event `self.ReceiveBeginPlay`
  ;[1 1 1] side to side platform
  (bind _output_get (set `self.originalLocation` (`self.K2_GetActorLocation`)))
  (set `self.newLocation` (+ _output_get (`KismetMathLibrary.MakeVector` (`self.x movement`))))
  (`TimelineComponent.SetPlayRate` (`self.Moveside`) (`self.speed`))
  (bind (_direction _moveup) (`Timeline|Moveside` :!via `PlayFromStart`)
    (:`Update`
      (`self.K2_SetActorLocation` (`KismetMathLibrary.VLerp` (`self.originalLocation`) (`self.newLocation`) _moveup)))))

(fn `UserConstructionScript`)