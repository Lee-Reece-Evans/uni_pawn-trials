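; BP_enemyAI is a side-scroller enemy that chases the player and explodes on contact, dealing damage.
; It turns to face the player each tick and uses PawnSensing, with a configurable sight radius, to trigger AIMoveTo.
; Overlapping the player destroys it, spawns explosion effects at the player and calls DamagePlayer.
; DamageAI reduces health; at zero it ragdolls, disables capsule collision and adds score through MyGameMode.
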(event `self.ReceiveBeginPlay`
  ;[1 1 1] set sight range
  (set `PawnSensingComponent.SightRadius` (`self.SightRange`) (`self.PawnSensing`)))

(event `DamageAI`
  (params (Damage :type "Float (double-precision)"))
  ;[1 1 1] take damage / death sequence & increase player score
  (set `self.Health` (- (`self.Health`) Damage))
  (if (<= (`self.Health`) 0.0)
    (set `self.isdead` true)
    (`PrimitiveComponent.SetSimulatePhysics` (`self.Mesh`) true)
    (`MovementComponent.StopMovementImmediately` (`self.CharacterMovement`))
    (`PrimitiveComponent.SetCollisionEnabled` (`self.CapsuleComponent`) "NoCollision")
    (bind _asmy_game_mode (cast `/Game/Blueprints/GameMode/MyGameMode` (`GameplayStatics.GetGameMode`)))
    (`/Game/Blueprints/GameMode/MyGameMode.IncScore` _asmy_game_mode (`self.score`))))

(event `self.ReceiveTick`
  (params (DeltaSeconds :type "Float (single-precision)"))
  ;[1 1 1] keep ai facing player
  (if (not (`self.isdead`))
    (`self.K2_SetActorRotation` (`KismetMathLibrary.MakeRotator` 0.0 0.0 (.yaw (`KismetMathLibrary.FindLookAtRotation` (`self.K2_GetActorLocation`) (`self.K2_GetActorLocation` (`GameplayStatics.GetPlayerCharacter` 0))))))))

(event `self.PawnSensing.OnSeePawn`
  (params (Pawn :type "Pawn Object Reference"))
  ;[1 1 1] move to player
  (if (not (`self.isdead`))
    (bind _asside_scroller_character_two (cast `/Game/Blueprints/SideScrollerCharacterTwo` Pawn))
    (`|AIMoveTo` self (0.0 0.0 0.0) _asside_scroller_character_two)))

(event `self.ReceiveActorBeginOverlap`
  (params (OtherActor :type "Actor Object Reference"))
  (bind _returnvalue (`self.K2_GetActorLocation` (`GameplayStatics.GetPlayerCharacter` 0)))
  ;[1 1 1] damage on impact
  (cast `/Game/Blueprints/SideScrollerCharacterTwo` OtherActor)
  (`self.K2_DestroyActor`)
  (`GameplayStatics.SpawnEmitterAtLocation` "/Game/StarterContent/Particles/P_Explosion.P_Explosion" _returnvalue)
  (`GameplayStatics.PlaySoundAtLocation` "/Game/StarterContent/Audio/Explosion_Cue.Explosion_Cue" _returnvalue (struct) 1.0 1.0 0.0 null null null)
  (bind _asside_scroller_character_two (cast `/Game/Blueprints/SideScrollerCharacterTwo` (`GameplayStatics.GetPlayerCharacter` 0)))
  (`/Game/Blueprints/SideScrollerCharacterTwo.DamagePlayer` _asside_scroller_character_two (`self.Damage`)))

(fn `UserConstructionScript`)