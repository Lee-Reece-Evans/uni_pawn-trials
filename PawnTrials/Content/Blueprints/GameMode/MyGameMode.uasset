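; MyGameMode is a game mode that tracks the score and elapsed time of the current game.
; On BeginPlay it caches MyGameInstance, and Tick accumulates GameTime until GameOver is set.
; IncScore adds a collectable's value to both the local Score and the game instance's TotalScore.
; GetScoreText and GetTimeText format score and whole seconds as text.
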(event `self.ReceiveBeginPlay`
  ;[1 1 1] get game instance
  (bind _asmy_game_instance (cast `/Game/Blueprints/GameMode/MyGameInstance` (`GameplayStatics.GetGameInstance`))
    (:`then`
      (set `self.GameInstance` _asmy_game_instance))
    (:`CastFailed`
      (`KismetSystemLibrary.PrintString` "CANT FIND GAME INSTANCE"))))

(event `self.ReceiveTick`
  (params (DeltaSeconds :type "Float (single-precision)"))
  ;[1 1 1] game time
  (if (not (`self.GameOver`))
    (set `self.GameTime` (+ DeltaSeconds (`self.GameTime`)))))

(event `IncScore`
  (params (Amount :type Integer))
  (bind _gameinstance (`self.GameInstance`))
  ;[1 1 1] increase score
  (set `self.CollectableValue` Amount)
  (set `self.Score` (+ (`self.CollectableValue`) (`self.Score`)))
  (set `/Game/Blueprints/GameMode/MyGameInstance.TotalScore` (+ (`self.CollectableValue`) (`/Game/Blueprints/GameMode/MyGameInstance.TotalScore` _gameinstance)) _gameinstance))

(fn `get score text`
  (returns (`return value` :type Text))
  (return (`KismetTextLibrary.Conv_IntToText` (`self.Score`))))

(fn `get time text`
  (returns (`return value` :type Text))
  (return (`KismetTextLibrary.Conv_StringToText` (`KismetStringLibrary.Concat_StrStr` (`KismetStringLibrary.Conv_IntToString` (`KismetMathLibrary.FFloor` (`self.GameTime`))) "s"))))

(fn `UserConstructionScript`)