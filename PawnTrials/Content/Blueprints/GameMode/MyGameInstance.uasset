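; Game instance that persists per-level best scores and times across levels and sessions.
; On Init it loads BP_saveGame from the save slot into its BestScore and BestTime arrays, or creates and writes a new save when none exists.
; A save event copies both arrays back to the slot.
; Two getters format the current LevelNum entries as text, appending "s" to the time.
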(event `self.ReceiveInit`
  ;[1 1 1] check save game exsits and load data if not create save (unreal save/load documentation)
  (bind _returnvalue (`GameplayStatics.DoesSaveGameExist` (`self.save game slot`)))
  (if _returnvalue
    (bind _returnvalue_2 (`GameplayStatics.LoadGameFromSlot` (`self.save game slot`)))
    (bind _output_get (set `self.save game ref` _returnvalue_2))
    (bind _asbp_save_game (cast `/Game/Blueprints/BP_savegame` _output_get))
    (`|ExecutionSequence`
      (:`then_0`
        (set `self.best time` (`/Game/Blueprints/BP_savegame.best time` _asbp_save_game)))
      (:`then_1`
        (set `self.best score` (`/Game/Blueprints/BP_savegame.best score` _asbp_save_game))))
    (else
      (bind _returnvalue_3 (`GameplayStatics.CreateSaveGameObject` "/Game/Blueprints/BP_savegame.BP_saveGame_C"))
      (bind _output_get_2 (set `self.save game ref` _returnvalue_3))
      (bind _asbp_save_game_2 (cast `/Game/Blueprints/BP_savegame` _output_get_2))
      (`|ExecutionSequence`
        (:`then_0`
          (set `/Game/Blueprints/BP_savegame.best score` (`self.best score`) _asbp_save_game_2))
        (:`then_1`
          (set `/Game/Blueprints/BP_savegame.best time` (`self.best time`) _asbp_save_game_2))
        (:`then_2`
          (`GameplayStatics.SaveGameToSlot` _output_get_2 (`self.save game slot`)))))))

(event `save`
  ;[1 1 1] save game data (unreal save / load documentation)
  (bind _asbp_save_game (cast `/Game/Blueprints/BP_savegame` (`self.save game ref`)))
  (`|ExecutionSequence`
    (:`then_0`
      (set `/Game/Blueprints/BP_savegame.best score` (`self.best score`) _asbp_save_game))
    (:`then_1`
      (set `/Game/Blueprints/BP_savegame.best time` (`self.best time`) _asbp_save_game))
    (:`then_2`
      (`GameplayStatics.SaveGameToSlot` _asbp_save_game (`self.save game slot`)))))

(fn `get best score text`
  (returns (`return value` :type Text))
  ;[1 1 1] best score text
  (return (`KismetTextLibrary.Conv_IntToText` (`|GetArrayItem` (`self.best score`) (`self.level num`)))))

(fn `get best time text`
  (returns (`return value` :type Text))
  ;[1 1 1] get best time text
  (return (`KismetTextLibrary.Conv_StringToText` (`KismetStringLibrary.Concat_StrStr` (`KismetStringLibrary.Conv_IntToString` (`|GetArrayItem` (`self.best time`) (`self.level num`))) "s"))))