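; BP_fireTrap is a trap that alternates fire between two spawn points.
; From BeginPlay it loops endlessly, spawning a BP_trapFlame at Spawnpoint1, destroying it after the AlternateSpeed delay, then doing the same at Spawnpoint2.
; The trap passes its Damage and DamageRate values to each flame on spawn, and toggles fire by recreating actors rather than reusing them.
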(event `self.ReceiveBeginPlay`
  (bind _alternate_speed (`self.Alternate Speed`))
  (bind _damage_rate (`self.Damage Rate`))
  (bind _damage (`self.Damage`))
  ;[1 1 1] alternate fire spawning points
  (bind _returnvalue (`|SpawnActorFromClass` "/Game/Blueprints/BP_trapFlame.BP_trapFlame_C" (`SceneComponent.K2_GetComponentToWorld` (`self.Spawnpoint1`)) "Undefined" "OverrideRootScale" null _damage_rate _damage null :!label _label))
  (`KismetSystemLibrary.Delay` _alternate_speed)
  (`self.K2_DestroyActor` _returnvalue)
  (bind _returnvalue_2 (`|SpawnActorFromClass` "/Game/Blueprints/BP_trapFlame.BP_trapFlame_C" (`SceneComponent.K2_GetComponentToWorld` (`self.Spawnpoint2`)) "Undefined" "OverrideRootScale" null _damage_rate _damage null))
  (`KismetSystemLibrary.Delay` _alternate_speed)
  (`self.K2_DestroyActor` _returnvalue_2)
  (goto _label))

(fn `UserConstructionScript`)