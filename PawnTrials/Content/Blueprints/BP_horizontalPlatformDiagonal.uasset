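; BP_horizontalPlatformDiagonal is a moving platform that travels along a straight line in the Y-Z plane, allowing diagonal motion.
; On BeginPlay it stores its start location and adds the Y and Z movement offsets to get the target.
; The Moveside timeline, played at a rate set by Speed, lerps the actor between the two points each update, without sweeping.
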(event `self.ReceiveBeginPlay`
  ;[1 1 1] forward / backwards platform
  (bind _output_get (set `self.originalLocation` (`self.K2_GetActorLocation`)))
  (set `self.newLocation` (+ _output_get (`KismetMathLibrary.MakeVector` 0.0 (`self.y movement`) (`self.z movement`))))
  (`TimelineComponent.SetPlayRate` (`self.Moveside`) (`self.speed`))
  (bind (_direction _moveup) (`Timeline|Moveside` :!via `PlayFromStart`)
    (:`Update`
      (`self.K2_SetActorLocation` (`KismetMathLibrary.VLerp` (`self.originalLocation`) (`self.newLocation`) _moveup)))))

(fn `UserConstructionScript`)